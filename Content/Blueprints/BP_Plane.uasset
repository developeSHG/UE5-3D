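; BP_Plane is a player-controllable plane that flies forward continuously and rolls in response to input.
; Tick moves the actor along its forward vector at MoveSpeed, scaled by delta time, without sweeping for collisions.
; The Turn axis applies a frame-rate-independent local roll to the Body component at RotateSpeed, with no yaw or pitch change.
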(event EventBeginPlay)

(event EventTick
  (params (DeltaSeconds :type Float%20%28single-precision%29))
  (Transformation|SetActorLocation (+ (Transformation|GetActorLocation) (* (Transformation|GetActorForwardVector) (* (Variables|Default|GetMoveSpeed) DeltaSeconds))) false false))

(event Input|AxisEvents|InputAxisTurn
  (params (AxisValue :type Float%20%28single-precision%29))
  (if (!= AxisValue 0.0)
    (Transformation|AddLocalRotation (Variables|Default|GetBody) (Math|Rotator|MakeRotator (* AxisValue (* (Variables|Default|GetRotateSpeed) (Utilities|Time|GetWorldDeltaSeconds))) 0.0 0.0) false false)))

(fn ConstructionScript)